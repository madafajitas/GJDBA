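; BP_Drone_Taser is a flying enemy drone that patrols points and chases BP_Ema on sight.
; Patrullar moves through PuntosDePatrulla via direct AI moves without pathfinding, timing each leg by distance rather than arrival.
; PawnSensing switches state, turns the spotlight red and raises speed, while a retriggerable delay restores blue patrol after lost sight.
; Capsule contact with Ema opens Lvl_Ema.
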(event `self.PawnSensing.OnSeePawn`
  (params (Pawn :type "Pawn Object Reference"))
  (bind _asbp_ema (cast `/Game/Pj_Drone/BP_Ema` Pawn))
  (set `self.EstadoActual` "NewEnumerator1")
  (`LightComponent.SetLightColor` (`self.SpotLight`) (struct :`R` 0.869792 :`G` 0.000418 :`B` 0.003554 :`A` 1.0) true)
  (set `CharacterMovementComponent.MaxFlySpeed` 900.0 (`self.CharacterMovement`))
  (`AIController.MoveToActor` (`AIBlueprintHelperLibrary.GetAIController` self) _asbp_ema 50.0 true false true null true)
  (`KismetSystemLibrary.RetriggerableDelay` 3.0)
  (`AIController.K2_ClearFocus` (`AIBlueprintHelperLibrary.GetAIController` self))
  (set `self.EstadoActual` "NewEnumerator0")
  (`LightComponent.SetLightColor` (`self.SpotLight`) (struct :`R` 0.000638 :`G` 0.039984 :`B` 0.604167 :`A` 1.0) true)
  (set `CharacterMovementComponent.MaxFlySpeed` 600.0 (`self.CharacterMovement`))
  (`self.Patrullar`))

(event `self.ReceiveBeginPlay`
  (`CharacterMovementComponent.SetMovementMode` (`self.CharacterMovement`) "MOVE_Flying" 0)
  (`self.Patrullar`))

(event `Patrullar`
  (bind _output (`|GetArrayItem` (`self.PuntosDePatrulla`) (`self.IndiceActual`)))
  (if (`|EnumEquality` (`self.EstadoActual`) "NewEnumerator0")
    (`/Engine/EditorBlueprintResources/StandardMacros.IsValid` _output
      (:`Is Valid`
        (`AIController.MoveToActor` (`AIBlueprintHelperLibrary.GetAIController` self) _output 100.0 true false true null true)
        (`KismetSystemLibrary.Delay` (+ (/ (`KismetMathLibrary.Vector_Distance` (`self.K2_GetActorLocation`) (`self.K2_GetActorLocation` _output)) 600.0) 2.0))
        (bind _result (`/Engine/EditorBlueprintResources/StandardMacros.IncrementInt` (`self.IndiceActual`))
          (:`  `
            (if (>= (`KismetArrayLibrary.Array_Length` (`self.PuntosDePatrulla`)) (`self.IndiceActual`))
              (set `self.IndiceActual` _result))
            (`self.Patrullar`)))))))

(event `self.CapsuleComponent.OnComponentHit`
  (params (HitComponent :type "PrimitiveComponent Object Reference") (OtherActor :type "Actor Object Reference") (OtherComp :type "PrimitiveComponent Object Reference") (NormalImpulse :type "Vector Structure") (Hit :type "HitResult Structure (by ref)"))
  (cast `/Game/Pj_Drone/BP_Ema` OtherActor)
  (`GameplayStatics.OpenLevel` "Lvl_Ema"))

(fn `UserConstructionScript`)