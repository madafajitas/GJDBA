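; BP_Drone_Taser is a flying drone Character with an unfinished patrol setup.
; On BeginPlay it enters Flying mode, prints the patrol point count and calls IrAlSiguientePunto.
; That event issues an AI MoveToActor without pathfinding, but no goal is wired in.
; The delayed, wrapping index advance is disconnected, so the patrol never cycles, and no taser logic is present.
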(event `self.ReceiveBeginPlay`
  (`CharacterMovementComponent.SetMovementMode` (`self.CharacterMovement`) "MOVE_Flying" 0)
  (`KismetSystemLibrary.PrintString` (`KismetStringLibrary.Conv_IntToString` (`KismetArrayLibrary.Array_Length` (`self.PuntosDePatrulla`))))
  (`self.IrAlSiguientePunto`))

(event `IrAlSiguientePunto`
  (`AIController.MoveToActor` (`AIBlueprintHelperLibrary.GetAIController` self) null 100.0 true false true null true))

(fn `UserConstructionScript`)