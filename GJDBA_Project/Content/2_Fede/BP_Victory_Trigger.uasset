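; BP_Victory_Trigger is a level trigger that ends the game with a victory screen when its box is overlapped.
; The Box overlap event passes the other actor through CheckPlayer, then creates the WI_Victory widget and shows it.
; After a short delay it hides the widget, deletes the Slot_1 save game and opens Menu_Level.
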(event `self.Box.OnComponentBeginOverlap`
  (params (OverlappedComponent :type "PrimitiveComponent Object Reference") (OtherActor :type "Actor Object Reference") (OtherComp :type "PrimitiveComponent Object Reference") (OtherBodyIndex :type Integer) (bFromSweep :type Boolean) (SweepResult :type "HitResult Structure (by ref)"))
  ; Activa por box collision
  (`/Game/2_Fede/ML_Macros.CheckPlayer` OtherActor)
  (bind _returnvalue (`|CreateWidget` "/Game/2_Fede/WI_Victory.WI_Victory_C"))
  (bind _output_get (set `self.Win_Canvas` _returnvalue))
  (`UserWidget.AddToViewport` _output_get 0)
  (`Widget.SetVisibility` (`self.Win_Canvas`) "Visible")
  (`KismetSystemLibrary.Delay` 5.0)
  (`Widget.SetVisibility` (`self.Win_Canvas`) "Hidden")
  (`GameplayStatics.DeleteGameInSlot` "Slot_1")
  (`GameplayStatics.OpenLevel` "Menu_Level"))

(fn `UserConstructionScript`)