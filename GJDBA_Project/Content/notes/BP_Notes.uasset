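; Trigger actor that fades a note image onto the screen while the player character is inside its box.
; On BeginPlay it creates its own WBP_Notes widget, which it adds to the viewport on player overlap.
; Index selects one of four widget images, whose opacity a Fade timeline drives through ShowImage.
; On exit, a separate timeline played in reverse drives HideImage, with no removal of the widget from the viewport.
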(event `self.ReceiveBeginPlay`
  (bind _returnvalue (`|CreateWidget` "/Game/0_Puli/WBP_Notes.WBP_Notes_C"))
  (set `self.Hud_Ref` _returnvalue))

(event `self.Box.OnComponentBeginOverlap`
  (params (OverlappedComponent :type "PrimitiveComponent Object Reference") (OtherActor :type "Actor Object Reference") (OtherComp :type "PrimitiveComponent Object Reference") (OtherBodyIndex :type Integer) (bFromSweep :type Boolean) (SweepResult :type "HitResult Structure (by ref)"))
  (bind _hud_ref (`self.Hud_Ref`))
  (bind _hud_ref_2 (`self.Hud_Ref`))
  (bind _hud_ref_3 (`self.Hud_Ref`))
  (bind _hud_ref_4 (`self.Hud_Ref`))
  (if (== OtherActor (`GameplayStatics.GetPlayerCharacter` 0))
    (`UserWidget.AddToViewport` (`self.Hud_Ref`) 0)
    (bind (_direction _newtrack_0) (`Timeline|Fade` :!via `PlayFromStart`)
      (:`Update`
        (switch `int` (`self.Index`)
          (:`0`
            (`/Game/0_Puli/WBP_Notes.ShowImage` _hud_ref_4 (`/Game/0_Puli/WBP_Notes.Image_0` _hud_ref_4) _newtrack_0))
          (:`1`
            (`/Game/0_Puli/WBP_Notes.ShowImage` _hud_ref (`/Game/0_Puli/WBP_Notes.Image_1` _hud_ref) _newtrack_0))
          (:`2`
            (`/Game/0_Puli/WBP_Notes.ShowImage` _hud_ref_2 (`/Game/0_Puli/WBP_Notes.Image_2` _hud_ref_2) _newtrack_0))
          (:`3`
            (`/Game/0_Puli/WBP_Notes.ShowImage` _hud_ref_3 (`/Game/0_Puli/WBP_Notes.Image_3` _hud_ref_3) _newtrack_0)))))))

(event `self.Box.OnComponentEndOverlap`
  (params (OverlappedComponent :type "PrimitiveComponent Object Reference") (OtherActor :type "Actor Object Reference") (OtherComp :type "PrimitiveComponent Object Reference") (OtherBodyIndex :type Integer))
  (bind _hud_ref (`self.Hud_Ref`))
  (bind _hud_ref_2 (`self.Hud_Ref`))
  (bind _hud_ref_3 (`self.Hud_Ref`))
  (bind _hud_ref_4 (`self.Hud_Ref`))
  (if (== OtherActor (`GameplayStatics.GetPlayerCharacter` 0))
    (bind (_direction _newtrack_0) (`Timeline|Timeline` :!via `ReverseFromEnd`)
      (:`Update`
        (switch `int` (`self.Index`)
          (:`0`
            (`/Game/0_Puli/WBP_Notes.HideImage` _hud_ref (`/Game/0_Puli/WBP_Notes.Image_0` _hud_ref) _newtrack_0))
          (:`1`
            (`/Game/0_Puli/WBP_Notes.HideImage` _hud_ref_3 (`/Game/0_Puli/WBP_Notes.Image_1` _hud_ref_3) _newtrack_0))
          (:`2`
            (`/Game/0_Puli/WBP_Notes.HideImage` _hud_ref_4 (`/Game/0_Puli/WBP_Notes.Image_2` _hud_ref_4) _newtrack_0))
          (:`3`
            (`/Game/0_Puli/WBP_Notes.HideImage` _hud_ref_2 (`/Game/0_Puli/WBP_Notes.Image_3` _hud_ref_2) _newtrack_0)))))))

(fn `UserConstructionScript`)