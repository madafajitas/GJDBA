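; Climbable stair (ladder-like) actor that attaches BP_Player to itself and releases them at either end.
; UsingStair accepts a usable player who is walking or falling downward, snaps and turns them to the stair, switches to Flying and enables Roof collision.
; Exit requires proximity to Top or Bot, restores Falling and rotation settings, then plays the nearer end's timeline to nudge the player along world Y, with added lift at the top.
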(event `Set Roof Location`
  (bind (_returnvalue_x _returnvalue_y _returnvalue_z) (`KismetMathLibrary.BreakVector` (`SceneComponent.K2_GetComponentLocation` (`self.top`))))
  ; Ubica la posición de la colisión, para que no se vea alterada por la escala del objeto
  (`SceneComponent.K2_SetWorldLocation` (`self.Roof`) (`KismetMathLibrary.MakeVector` _returnvalue_x _returnvalue_y (+ _returnvalue_z (`self.RoofZ Location`))) false false))

(event `self.ReceiveBeginPlay`
  ; Sacamos la Referencia del player y seteamos la colision del techo
  (bind _asbp_player (cast `/Game/0_Puli/BP_Puli/BP_Player` (`GameplayStatics.GetPlayerPawn` 0)))
  (set `self.As BP Player` _asbp_player)
  (`PrimitiveComponent.SetCollisionEnabled` (`self.Roof`) "NoCollision")
  (`self.Set Roof Location`))

(event `UsingStair`
  (bind (_returnvalue_x _returnvalue_y) (`KismetMathLibrary.BreakVector` (`self.K2_GetActorLocation`)))
  (bind _as_bp_player (`self.As BP Player`))
  (bind _as_bp_player_2 (`self.As BP Player`))
  (bind (_returnvalue_x_2 _returnvalue_y_2 _returnvalue_z) (`KismetMathLibrary.BreakVector` (`self.K2_GetActorLocation` _as_bp_player)))
  (bind _charactermovement (`Character.CharacterMovement` _as_bp_player))
  (bind _charactermovement_2 (`Character.CharacterMovement` _as_bp_player_2))
  (bind (_returnvalue_roll _returnvalue_pitch _returnvalue_yaw) (`KismetMathLibrary.BreakRotator` (`KismetMathLibrary.FindLookAtRotation` (`self.K2_GetActorLocation` _as_bp_player) (`self.K2_GetActorLocation`))))
  (bind _movementmode (`CharacterMovementComponent.MovementMode` _charactermovement_2))
  (bind (_velocity_x _velocity_y _velocity_z) (`KismetMathLibrary.BreakVector` (`MovementComponent.Velocity` _charactermovement_2)))
  ; Si se cumplen una serie de condiciones, pasamos a estar en la escalera
  (if (`/Game/0_Puli/BP_Puli/BP_Player.canUse` _as_bp_player_2)
    (if (`|EnumEquality` _movementmode "MOVE_Walking")
      ; Ponemos al Player en la escalera y activamos la colision del techo
      (set `/Game/0_Puli/BP_Puli/BP_Player.onStair` true _as_bp_player :!label _label)
      (`PrimitiveComponent.SetCollisionEnabled` (`self.Roof`) "QueryAndPhysics")
      (`self.K2_SetActorLocation` _as_bp_player (+ (`KismetMathLibrary.MakeVector` _returnvalue_x _returnvalue_y _returnvalue_z) (* (`self.GetActorForwardVector`) 10.0) (`KismetMathLibrary.MakeVector` (* (`self.XOffset`) -1.0) (* (`self.YOffset`) -1.0) (* (`self.ZOffset`) -1.0))) false false)
      ; Rotamos al Player para que mire hacia la escalera
      (`self.K2_SetActorRotation` _as_bp_player (`KismetMathLibrary.MakeRotator` 0.0 0.0 _returnvalue_yaw) false)
      ; Cambiamos el Movement Mode, lo dejamos quieto y le sacamos la orientación de rotación
      (`CharacterMovementComponent.SetMovementMode` _charactermovement "MOVE_Flying" 0)
      (`MovementComponent.StopMovementImmediately` _charactermovement)
      (set `CharacterMovementComponent.bOrientRotationToMovement` false _charactermovement)
      (elif (and (`|EnumEquality` _movementmode "MOVE_Falling") (< _velocity_z 0.0))
        (goto _label)))))

(event `Exit`
  (bind _as_bp_player (`self.As BP Player`))
  (bind _as_bp_player_2 (`self.As BP Player`))
  (bind _as_bp_player_3 (`self.As BP Player`))
  (bind _charactermovement (`Character.CharacterMovement` _as_bp_player_2))
  ; Calculamos la distancia de interacción
  (`self.CanInteract`)
  (if (`self.OnRangeToInteract`)
    ; Volvemos a poner configuraciones al default
    (`PrimitiveComponent.SetCollisionEnabled` (`self.Roof`) "NoCollision")
    (`CharacterMovementComponent.SetMovementMode` _charactermovement "MOVE_Falling" 0)
    (set `/Game/0_Puli/BP_Puli/BP_Player.onStair` false _as_bp_player_2)
    (set `CharacterMovementComponent.bOrientRotationToMovement` true _charactermovement)
    ; Dependiendo de si estamos más cerca del piso o del techo, ejecutamos un movimiento u otro
    (`self.IsTopClosestPoint`)
    (if (`self.TopExit`)
      (bind (_direction _newtrack_0) (`Timeline|Timeline` :!via `PlayFromStart`)
        (:`Update`
          (`self.K2_SetActorLocation` _as_bp_player_3 (+ (`KismetMathLibrary.MakeVector` 0.0 _newtrack_0 1.5) (`self.K2_GetActorLocation` _as_bp_player_3)) false false)))
      (else
        (bind (_direction_2 _newtrack_0_2) (`Timeline|ExitBottom` :!via `PlayFromStart`)
          (:`Update`
            (`self.K2_SetActorLocation` _as_bp_player (+ (`KismetMathLibrary.MakeVector` 0.0 _newtrack_0_2) (`self.K2_GetActorLocation` _as_bp_player)) false false)))))))

(event `CanInteract`
  (bind _interactdistance (`self.InteractDistance`))
  (bind _returnvalue (`self.K2_GetActorLocation` (`self.As BP Player`)))
  ; Calculamos si estamos en distancia para interactuar
  (if (or (<= (`KismetMathLibrary.Vector_Distance` (`SceneComponent.K2_GetComponentLocation` (`self.top`)) _returnvalue) _interactdistance) (<= (`KismetMathLibrary.Vector_Distance` _returnvalue (`SceneComponent.K2_GetComponentLocation` (`self.bot`))) _interactdistance))
    (set `self.OnRangeToInteract` true)
    (else
      (set `self.OnRangeToInteract` false))))

(event `IsTopClosestPoint`
  (bind _returnvalue (`self.K2_GetActorLocation` (`self.As BP Player`)))
  ; Calculamos si estamos más cerca de la parte alta o de la parte baja
  (set `self.TopExit` (< (`KismetMathLibrary.Vector_Distance` (`SceneComponent.K2_GetComponentLocation` (`self.top`)) _returnvalue) (`KismetMathLibrary.Vector_Distance` _returnvalue (`SceneComponent.K2_GetComponentLocation` (`self.bot`))))))

(fn `UserConstructionScript`)