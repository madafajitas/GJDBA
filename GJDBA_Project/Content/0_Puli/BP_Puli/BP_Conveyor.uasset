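; BP_Conveyor is a conveyor belt that carries the player and BP_Box actors resting on it.
; Overlap begin and end events maintain an array of boxes and a flag for the player, whose pawn is cached on BeginPlay.
; Each Tick, Slide offsets those actors along the negated forward vector of BPConveyor, scaled by Speed and delta time, without sweeping.
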(event `self.ReceiveBeginPlay`
  ; Casteamos al player
  (bind _asbp_player (cast `/Game/0_Puli/BP_Puli/BP_Player` (`GameplayStatics.GetPlayerPawn` 0)))
  (set `self.Player_Ref` _asbp_player))

(event `self.ReceiveActorBeginOverlap`
  (params (OtherActor :type "Actor Object Reference"))
  ; Agregamos la caja que entro en el overlap a un array. También nos fijamos si el player entro al overlap y setteamos isPlayerOnOverlap = true
  (`|ExecutionSequence`
    (:`then_0`
      (bind _asbp_box (cast `/Game/0_Puli/BP_Puli/BP_Box` OtherActor))
      (set `self.isValidated` true)
      (`KismetArrayLibrary.Array_Add` (`self.BoxOnConveyor_Array`) _asbp_box))
    (:`then_1`
      (if (== OtherActor (`self.Player_Ref`))
        (set `self.isPlayerOnConveyor` true)))))

(event `self.ReceiveActorEndOverlap`
  (params (OtherActor :type "Actor Object Reference"))
  ; Si una caja dejo de overlapear, la sacamos del array. Si el player dejo de overlappear, isPlayerOnConveyor = false
  (`|ExecutionSequence`
    (:`then_0`
      (bind _asbp_box (cast `/Game/0_Puli/BP_Puli/BP_Box` OtherActor))
      (`KismetArrayLibrary.Array_RemoveItem` (`self.BoxOnConveyor_Array`) _asbp_box))
    (:`then_1`
      (if (== OtherActor (`self.Player_Ref`))
        (set `self.isPlayerOnConveyor` false)))))

(event `self.ReceiveTick`
  (params (DeltaSeconds :type "Float (single-precision)"))
  ; Movemos al player o a los elementos del array si estan encima
  (`|ExecutionSequence`
    (:`then_0`
      (if (`self.isPlayerOnConveyor`)
        (`self.Slide` (`self.Player_Ref`))))
    (:`then_1`
      (if (`self.isValidated`)
        (for _array_element (`self.BoxOnConveyor_Array`)
          (`self.Slide` _array_element))))))

(event `Slide`
  (params (ObjectToMove :type "Actor Object Reference"))
  ; Movemos un objeto a traves del frente de la masha
  (`self.K2_AddActorWorldOffset` ObjectToMove (* (`self.Speed`) (`GameplayStatics.GetWorldDeltaSeconds`) (* (`SceneComponent.GetForwardVector` (`self.BP_Conveyor`)) -1.0)) false false))

(fn `UserConstructionScript`)