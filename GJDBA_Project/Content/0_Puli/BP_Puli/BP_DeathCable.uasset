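; BP_DeathCable is a hazard actor that kills the player on contact.
; On BeginPlay it caches the player character as BP_Player.
; When that player overlaps it, the custom event Eldiablo plays a DroneZap 2D sound and calls Die on the player.
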(event `self.ReceiveBeginPlay`
  (bind _asbp_player (cast `/Game/0_Puli/BP_Puli/BP_Player` (`GameplayStatics.GetPlayerCharacter` 0)))
  (set `self.As BP Player` _asbp_player))

(event `self.ReceiveActorBeginOverlap`
  (params (OtherActor :type "Actor Object Reference"))
  (if (== OtherActor (`self.As BP Player`))
    (`self.Eldiablo`)))

(event `Eldiablo`
  (`GameplayStatics.PlaySound2D` "/Game/Sounds/Sound/droneZap.droneZap" 1.0 1.0 0.0 null null)
  (`/Game/0_Puli/BP_Puli/BP_Player.Die` (`self.As BP Player`)))

(fn `UserConstructionScript`)