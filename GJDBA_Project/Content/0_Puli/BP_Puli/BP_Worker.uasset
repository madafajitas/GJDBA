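; BP_Worker is a worker NPC that operates its assigned lever when called within ScreamRange of the player and can be freed within LiberationRange.
; ActivateLever uses AI MoveTo to reach and trigger the lever, returning the worker home if it was unsuccessful after its activation time.
; Liberation marks the worker freed once, decrements the GameMode's FreedWorkers counter and calls AllFreed.
; Sphere overlaps show and hide a scream-interaction hint widget.
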(event `self.ReceiveBeginPlay`
  ; Getting References
  (`/Engine/EditorBlueprintResources/StandardMacros.IsValid` (`self.Lever_Ref`)
    (:`Is Valid`
      (bind _asbp_player (cast `/Game/0_Puli/BP_Puli/BP_Player` (`GameplayStatics.GetPlayerPawn` 0)))
      (set `self.Player_Ref` _asbp_player)
      (bind _asgm_puli (cast `/Game/0_Puli/BP_Puli/CORE/GM_Puli` (`GameplayStatics.GetGameMode`)))
      (set `self.GM_Ref` _asgm_puli)
      (set `self.OriginalPosition` (`self.K2_GetActorLocation`)))
    (:`Is Not Valid`
      (`KismetSystemLibrary.PrintString` "Invalid Reference: Did you reference the lever in Details on every BP_Worker?" true true (struct :`R` 1.0 :`B` 0.006754 :`A` 1.0) 10.0))))

(event `ActivateLever`
  (bind _lever_ref (`self.Lever_Ref`))
  ;[0 0 0 0.5 36] Lever Activation
  ;; Checking if we are on hear range
  (if (<= (`self.GetDistanceTo` (`self.Player_Ref`)) (`self.ScreamRange`))
    (if (not (`self.ExecutingLever`))
      (set `self.ExecutingLever` true)
      ;; Going to lever on Listen
      (`|AIMoveTo` self (0.0 0.0 0.0) (`self.Lever_Ref`) 100.0
        (:`OnSuccess`
          ;; Once there, the lever is activated
          (`/Game/0_Puli/BP_Puli/BP_LeverTimed.RecieveActivation` _lever_ref)
          (set `self.playLeverAnim?` true)
          (`KismetSystemLibrary.Delay` 2.0)
          ;; If the door its not open after Activation Time, the Worker returns to its original position.
          (set `self.playLeverAnim?` false)
          (`KismetSystemLibrary.Delay` (`/Game/0_Puli/BP_Puli/BP_LeverTimed.ActivationTime` _lever_ref))
          (if (not (`/Game/0_Puli/BP_Puli/BP_LeverTimed.wasSuccesfull` _lever_ref))
            (`|AIMoveTo` self (`self.OriginalPosition`) null 50.0
              (:`OnSuccess`
                (set `self.ExecutingLever` false)))))))))

(event `Liberation`
  (bind _gm_ref (`self.GM_Ref`))
  ; Checking if we are on LiberationRange
  (if (<= (`self.GetDistanceTo` (`self.Player_Ref`)) (`self.LiberationRange`))
    (if (not (`self.isFreed`))
      ; On Liberation Range, checks if its already Freed and if its not, then freed the npc
      (bind _result (`/Engine/EditorBlueprintResources/StandardMacros.DecrementInt` (`/Game/0_Puli/BP_Puli/CORE/GM_Puli.FreedWorkers` _gm_ref))
        (:`  `
          (set `/Game/0_Puli/BP_Puli/CORE/GM_Puli.FreedWorkers` _result _gm_ref)
          (set `self.isFreed` true)
          (`/Game/0_Puli/BP_Puli/CORE/GM_Puli.AllFreed` _gm_ref))))))

(event `self.Sphere.OnComponentBeginOverlap`
  (params (OverlappedComponent :type "PrimitiveComponent Object Reference") (OtherActor :type "Actor Object Reference") (OtherComp :type "PrimitiveComponent Object Reference") (OtherBodyIndex :type Integer) (bFromSweep :type Boolean) (SweepResult :type "HitResult Structure (by ref)"))
  (if (== OtherActor (`GameplayStatics.GetPlayerCharacter` 0))
    (bind _returnvalue (`|CreateWidget` "/Game/0_Puli/WBP_Notes.WBP_Notes_C"))
    (`/Game/0_Puli/WBP_Notes.ScreamInteractText` _returnvalue)))

(event `self.Sphere.OnComponentEndOverlap`
  (params (OverlappedComponent :type "PrimitiveComponent Object Reference") (OtherActor :type "Actor Object Reference") (OtherComp :type "PrimitiveComponent Object Reference") (OtherBodyIndex :type Integer))
  (if (== OtherActor (`GameplayStatics.GetPlayerCharacter` 0))
    (`/Game/0_Puli/WBP_Notes.ScreamInteractLeave` (stale `self.Sphere.OnComponentBeginOverlap` _returnvalue))))

(fn `UserConstructionScript`)