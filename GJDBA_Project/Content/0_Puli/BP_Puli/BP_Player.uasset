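; Player character that moves, runs, climbs stairs, pauses the game and interacts with workers through Enhanced Input.
; Forward capsule-trace helpers find targets: a shout triggers a worker's lever on a short cooldown, while interact frees workers or toggles stair use via FlipFlop.
; Movement directions are hardcoded for the camera setup and switch to vertical input while OnStair, which is only cleared here.
; A notes trace helper exists but is not called here.
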(event `self.ReceiveActorBeginOverlap`
  (params (OtherActor :type "Actor Object Reference"))
  ; Obtenemos la referencia de la escalera al overlapear y nos fijamos si estamos a rango para interactuar
)

(event `self.ReceiveBeginPlay`
  ; Cambiando a mi MappingContext
  (message `EnhancedInputSubsystemInterface.AddMappingContext` (pcsubsystem `EnhancedInputLocalPlayerSubsystem` (`GameplayStatics.GetPlayerController` 0)) "/Game/0_Puli/MappingContext/IMC_PuliMC.IMC_PuliMC" 0 (struct)))

(event `EnhancedInput|/Game/0_Puli/MappingContext/IA_Scream`
  (params (ActionValue :type Boolean) (ElapsedSeconds :type "Float (double-precision)") (TriggeredSeconds :type "Float (double-precision)") (InputAction :type "InputAction Object Reference" :default "/Game/0_Puli/MappingContext/IA_Scream.IA_Scream"))
  ; Gritamos usando un trace buscando a Worker. Si lo casteamos activa la palanca. Podemos gritar cada xDelay.
  (:`Completed`
    (if (`self.canScream`)
      (set `self.canScream` false)
      (`GameplayStatics.PlaySound2D` "/Game/Sounds/Sound/characterHey.characterHey" 1.0 1.0 0.0 null null)
      (bind _asbp_worker (`self.Get BP_Worker`)
        (:`then`
          (`/Game/0_Puli/BP_Puli/BP_Worker.ActivateLever` _asbp_worker))
        (:`Faliled`
          _))
      (`KismetSystemLibrary.Delay` 0.3)
      (set `self.canScream` true))))

(event `EnhancedInput|/Game/0_Puli/MappingContext/IA_Interaction`
  (params (ActionValue :type Boolean) (ElapsedSeconds :type "Float (double-precision)") (TriggeredSeconds :type "Float (double-precision)") (InputAction :type "InputAction Object Reference" :default "/Game/0_Puli/MappingContext/IA_Interaction.IA_Interaction"))
  ; Usamos Trace para interactuar con la escalera o con un worker. La escalera usa un flip flop para subir y bajar. El trabajador debería activar una animación de sacar casco y luego liberar.
  (:`Completed`
    (`|ExecutionSequence`
      (:`then_0`
        (bind _as_bp_stairs (`self.Get_BP_Stair`)
          (:`OutExec`
            (`/Game/0_Puli/BP_Puli/BP_Stairs.CanInteract` _as_bp_stairs)
            (if (`/Game/0_Puli/BP_Puli/BP_Stairs.OnRangeToInteract` _as_bp_stairs)
              (`/Engine/EditorBlueprintResources/StandardMacros.FlipFlop`
                (:`A`
                  (set `self.canUse` true)
                  (`/Game/0_Puli/BP_Puli/BP_Stairs.UsingStair` _as_bp_stairs))
                (:`B`
                  (set `self.canUse` false)
                  (`/Game/0_Puli/BP_Puli/BP_Stairs.Exit` _as_bp_stairs)
                  (set `self.onStair` false)))))))
      (:`then_1`
        (bind _asbp_worker (`self.Get BP_Worker`)
          (:`then`
            (`/Game/0_Puli/BP_Puli/BP_Worker.Liberation` _asbp_worker)))))))

(event `EnhancedInput|/Game/0_Puli/MappingContext/IA_Pause`
  (params (ActionValue :type Boolean) (ElapsedSeconds :type "Float (double-precision)") (TriggeredSeconds :type "Float (double-precision)") (InputAction :type "InputAction Object Reference" :default "/Game/0_Puli/MappingContext/IA_Pause.IA_Pause"))
  (bind _returnvalue (`GameplayStatics.GetPlayerController` 0))
  (bind _returnvalue_2 (`GameplayStatics.GetPlayerController` 0))
  ; Sistema de Pausa
  (:`Started`
    (if (`self.isPaused`)
      (set `self.isPaused` false)
      (`Widget.RemoveFromParent` (`self.Pause_REf`))
      (`GameplayStatics.SetGamePaused` false)
      (`WidgetBlueprintLibrary.SetInputMode_GameOnly` _returnvalue)
      (set `PlayerController.bShowMouseCursor` false _returnvalue)
      (else
        (set `self.isPaused` true)
        (bind _returnvalue_3 (`|CreateWidget` "/Game/0_Puli/BP_Puli/UI/WBP_Pause.WBP_Pause_C" _returnvalue_2))
        (bind _output_get (set `self.Pause_REf` _returnvalue_3))
        (`UserWidget.AddToViewport` _output_get 0)
        (`WidgetBlueprintLibrary.SetInputMode_GameAndUIEx` _returnvalue_2 (`self.Pause_REf`))
        (set `PlayerController.bShowMouseCursor` true _returnvalue_2)
        (`GameplayStatics.SetGamePaused` true)))))

(event `EnhancedInput|/Game/Input/Actions/IA_Move`
  (params (ActionValue :type "Vector2D Structure") (ElapsedSeconds :type "Float (double-precision)") (TriggeredSeconds :type "Float (double-precision)") (InputAction :type "InputAction Object Reference" :default "/Game/Input/Actions/IA_Move.IA_Move"))
  (bind (_returnvalue_roll _returnvalue_pitch) (`KismetMathLibrary.BreakRotator` (`self.GetControlRotation`)))
  ; Movimiento hardcodeado en base a la nueva cámara (si editan la posición de la cámara, hay que modificar esto). También se agrega un tipo de movimiento si estamos en la escalera
  (:`Triggered`
    (if (`self.onStair`)
      (`self.StairMovement` ActionValue_Y)
      (else
        (`self.AddMovementInput` (`KismetMathLibrary.GetRightVector` (`KismetMathLibrary.MakeRotator` 0.0 _returnvalue_pitch)) ActionValue_Y)
        (`self.AddMovementInput` (* (`KismetMathLibrary.GetForwardVector` (`KismetMathLibrary.MakeRotator` 0.0)) -1.0) ActionValue_X))))
  (:`Completed`
    (`MovementComponent.StopMovementImmediately` (`self.CharacterMovement`))))

(event `StairMovement`
  (params (`Y axis` :type "Float (double-precision)"))
  ; Movimiento de escalera. W es para arriba y S para abajo, colta
  (`self.AddMovementInput` (`self.GetActorUpVector`) `Y axis`))

(event `Key|LeftShift`
  (params (Key :type "Key Structure"))
  ; Correr con shift o caminar al soltarlo
  (:`Pressed`
    (set `CharacterMovementComponent.MaxWalkSpeed` (`self.RunSpeed`) (`self.CharacterMovement`)))
  (:`Released`
    (set `CharacterMovementComponent.MaxWalkSpeed` (`self.WalkSpeed`) (`self.CharacterMovement`))))

(fn `UserConstructionScript`)