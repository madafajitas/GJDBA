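; GM_Puli is a game mode that restores saved state on start and handles worker-rescue feedback and player death.
; BeginPlay loads Slot_1 into BP_SaveGame, moves the player pawn to the saved transform and applies the saved master volume through a sound mix.
; AllFreed prints either completion or the FreedWorkers count still to liberate.
; Death adds the WBP_Death widget to the viewport.
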(event `self.ReceiveBeginPlay`
  ; Hay que cambiar esto de lugar. Ahora se ejecuta despues del primer frame del juego, pero debería hacerse desde el inicio. Quizás en un menú prinipcal del juego. Lo de cargar la posición del jugador debería quedar acá
  (bind _returnvalue (`GameplayStatics.LoadGameFromSlot` "Slot_1"))
  (bind _asbp_save_game (cast `/Game/bp_Fede/BP_SaveGame` _returnvalue))
  (`self.K2_SetActorTransform` (`GameplayStatics.GetPlayerPawn` 0) (`/Game/bp_Fede/BP_SaveGame.PlayerPosition` _asbp_save_game) false false)
  (`GameplayStatics.SetSoundMixClassOverride` "/Game/Sounds/Attenuation/MasterVolume.MasterVolume" "/Engine/EngineSounds/Master.Master" (`/Game/bp_Fede/BP_SaveGame.VolumeValue` _asbp_save_game))
  (`GameplayStatics.PushSoundMixModifier` "/Game/Sounds/Attenuation/MasterVolume.MasterVolume"))

(event `AllFreed`
  (bind _freedworkers (`self.FreedWorkers`))
  ; Chequea si todos los trabajadores fueron liberados
  (if (<= _freedworkers 0)
    (`KismetSystemLibrary.PrintString` "Todos los humanos han sido liberados" true true (struct :`G` 1.0 :`B` 0.058628 :`A` 1.0) 3.0)
    (else
      (`KismetSystemLibrary.PrintString` (`KismetStringLibrary.Concat_StrStr` "Faltan liberar " (`KismetStringLibrary.Conv_IntToString` _freedworkers) " compañeros!") true true (struct :`R` 1.0 :`G` 0.952128 :`A` 1.0) 3.0))))

(event `Death`
  ; Metemos el Widget de perder
  (bind _returnvalue (`|CreateWidget` "/Game/0_Puli/BP_Puli/UI/WBP_Death.WBP_Death_C"))
  (`UserWidget.AddToViewport` _returnvalue 0))

(fn `UserConstructionScript`)