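; BP_Door is a door that opens once every lever in its per-instance, level-configured LeverArray is activated.
; BeginPlay only warns about invalid lever references; the CheckingLevers event scans the array, stops at the first inactive lever, and otherwise calls Open.
; Open marks each lever successful and, after a short delay, plays audio and a timeline that provisionally raises the door mesh along Z, scaled by AlturaMaxima.
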(event `self.ReceiveBeginPlay`
  ; Obtenemos un array de Levers configurable desde el editor de nivel
  (for _array_element (`self.Lever_Array`)
    (`/Engine/EditorBlueprintResources/StandardMacros.IsValid` _array_element
      (:`Is Not Valid`
        (`KismetSystemLibrary.PrintString` "Referencia Inválida: Referenció la palanca en Details de cada BP_Door?" true true (struct :`R` 1.0 :`B` 0.024787 :`A` 1.0) 5.0)))))

(event `CheckingLevers`
  ;[0 0 0 0.5 36] Chequeando el isActivated de cada Lever
  ;; Por cada bucle, revisamos si algun lever tiene su isActivated en falso. Si no lo tiene, seguimos el bucle. Si lo tiene, rompemos el bucle
  (for _array_element (`self.Lever_Array`)
    (bind _isactivated (`/Game/0_Puli/BP_Puli/BP_LeverTimed.isActivated` _array_element))
    (`KismetSystemLibrary.PrintString` (`KismetStringLibrary.Conv_BoolToString` _isactivated) true true (struct :`R` 0.718288 :`B` 1.0 :`A` 1.0))
    (bind _output_get (set `self.uno inactivo` (== _isactivated false)))
    (if _output_get
      (break)
      (else
        (`KismetSystemLibrary.PrintString` "Revisando siguiente Lever" true true (struct :`R` 0.718288 :`B` 1.0 :`A` 1.0)))))
  ;; Al completar el bucle, si ninguno de los Lever tuvo isActivated en false, entonces AllActive = true y pasamos a abrir la puerta
  (if (not (`self.uno inactivo`))
    (set `self.allActive` true)
    (`KismetSystemLibrary.PrintString` "Ninguno fue inactivo" true true (struct :`R` 0.385563 :`B` 1.0 :`A` 1.0))
    (`self.Open`)))

(event `Open`
  ; Setteamos WasSuccesfull de cada Lever en verdadero y como provisional, levantamos la puerta
  (for _array_element (`self.Lever_Array`)
    (set `/Game/0_Puli/BP_Puli/BP_LeverTimed.wasSuccesfull` true _array_element)
    (`KismetSystemLibrary.Delay` 0.5)
    (`AudioComponent.Play` (`self.DoorAudio`) 0.0)
    (bind (_direction _newtrack_0) (`Timeline|OpenDoor`)
      (:`Update`
        (`SceneComponent.K2_SetRelativeLocation` (`self.Box_E9E6F689`) (`KismetMathLibrary.MakeVector` 0.0 0.0 (* _newtrack_0 (`self.alturaMaxima`))) false false)))))

(fn `UserConstructionScript`)