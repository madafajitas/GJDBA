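; Pusher sweeper obstacle whose moving cube repeatedly slides out and back along local Y, launching the player away from the actor's origin on overlap.
; A timeline drives the offset by bar length at a configurable play rate, restarting after an interval delay.
; Each update also aims and Y-scales a pivot to stretch the connecting tube between base and moving cube.
; 2D sounds mark the push, return and steam at cycle end.
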(event `self.ReceiveBeginPlay`
  ; Cast al player e iniciamos la lógica de barrida
  (bind _asbp_player (cast `/Game/0_Puli/BP_Puli/BP_Player` (`GameplayStatics.GetPlayerPawn` 0)))
  (set `self.Player_Ref` _asbp_player)
  (set `self.InitialLocation` (`SceneComponent.RelativeLocation` (`self.CubeMovil`)))
  (`self.Sweep`))

(event `self.ReceiveActorBeginOverlap`
  (params (OtherActor :type "Actor Object Reference"))
  (bind _player_ref (`self.Player_Ref`))
  ; Calculamos por dónde chocamos al player y usamos esa dirección para empujarlo multiplicado por una fuerza
  (if (== OtherActor _player_ref)
    (bind _output_get (set `self.Direction` (`KismetMathLibrary.Normal` (- (`self.K2_GetActorLocation` _player_ref) (`self.K2_GetActorLocation`)))))
    (`Character.LaunchCharacter` _player_ref (* _output_get (`self.PushStrength`)) false false)))

(event `Sweep`
  (bind (_initiallocation_x _initiallocation_y) (`KismetMathLibrary.BreakVector` (`self.InitialLocation`)))
  ; Lógica de barrida. El cubo móvil va y vuelve mediante su locación con un delay.
  (`GameplayStatics.PlaySound2D` "/Game/Sounds/Cues/pushWall_Cue.pushWall_Cue" 1.0 1.0 0.0 null null)
  (bind (_direction _newtrack_0) (`Timeline|GoAndCome` :!via `PlayFromStart` :!label _label)
    (:`Update`
      (`SceneComponent.K2_SetRelativeLocation` (`self.CubeMovil`) (`KismetMathLibrary.MakeVector` 0.0 (+ (* _newtrack_0 (`self.barLenght`)) _initiallocation_y)) false false)
      (`self.Scale Connection`)
      (if (> (`TimelineComponent.GetPlaybackPosition` (`self.GoAndCome`)) 1.25)
        (if (`self.bCanPlayBackAudio`)
          (`GameplayStatics.PlaySound2D` "/Game/Sounds/Cues/pushWallBack_Cue.pushWallBack_Cue" 1.0 1.0 0.0 null null)
          (set `self.bCanPlayBackAudio` false))))
    (:`Finished`
      (`GameplayStatics.PlaySound2D` "/Game/Sounds/Cues/pushWallSteam_Cue.pushWallSteam_Cue" 1.0 1.0 0.0 null null)
      (`KismetSystemLibrary.Delay` (`self.IntervalDelay`))
      (`GameplayStatics.PlaySound2D` "/Game/Sounds/Cues/pushWall_Cue.pushWall_Cue" 1.0 1.0 0.0 null null)
      (set `self.bCanPlayBackAudio` true)
      (goto _label :!via `PlayFromStart`))))

(event `Scale Connection`
  (bind _pivot (`self.Pivot`))
  (bind _returnvalue (`SceneComponent.K2_GetComponentLocation` (`self.CubeBase`)))
  (bind (_returnvalue_x _returnvalue_y _returnvalue_z) (`KismetMathLibrary.BreakVector` (`SceneComponent.K2_GetComponentScale` _pivot)))
  (bind _returnvalue_2 (- _returnvalue (`SceneComponent.K2_GetComponentLocation` (`self.CubeMovil`))))
  ; Escalamos el "tubo" que conecta el cubo base con el cubo móvil, en base a su distancia
  (`SceneComponent.K2_SetWorldTransform` _pivot (`KismetMathLibrary.MakeTransform` _returnvalue (`KismetMathLibrary.MakeRotFromY` _returnvalue_2) (`KismetMathLibrary.MakeVector` _returnvalue_x (/ (`KismetMathLibrary.VSize` _returnvalue_2) 100.0) _returnvalue_z)) false false))

(fn `UserConstructionScript`
  (`TimelineComponent.SetPlayRate` (`self.GoAndCome`) (`self.Speed`)))