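; LadderCollision is a trigger actor that toggles a ladder interaction prompt when the player character enters or leaves its Box.
; On begin overlap, if the stored HUD reference is already valid, it replaces it with a newly created WBP_HUD and calls LadderInteractionText on it.
; The new widget is not added to the viewport here.
; On end overlap, it calls LadderInteractionLeave on the stored widget if valid.
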(event `self.Box.OnComponentBeginOverlap`
  (params (OverlappedComponent :type "PrimitiveComponent Object Reference") (OtherActor :type "Actor Object Reference") (OtherComp :type "PrimitiveComponent Object Reference") (OtherBodyIndex :type Integer) (bFromSweep :type Boolean) (SweepResult :type "HitResult Structure (by ref)"))
  (if (== OtherActor (`GameplayStatics.GetPlayerCharacter` 0))
    (`/Engine/EditorBlueprintResources/StandardMacros.IsValid` (`self.As WBP HUD`)
      (:`Is Valid`
        (bind _returnvalue (`|CreateWidget` "/Game/UI/HUD/WBP_HUD.WBP_HUD_C"))
        (bind _output_get (set `self.As WBP HUD` _returnvalue))
        (`/Game/UI/HUD/WBP_HUD.LadderInteractionText` _output_get)))))

(event `self.Box.OnComponentEndOverlap`
  (params (OverlappedComponent :type "PrimitiveComponent Object Reference") (OtherActor :type "Actor Object Reference") (OtherComp :type "PrimitiveComponent Object Reference") (OtherBodyIndex :type Integer))
  (if (== OtherActor (`GameplayStatics.GetPlayerCharacter` 0))
    (`/Engine/EditorBlueprintResources/StandardMacros.IsValid` (`self.As WBP HUD`)
      (:`Is Valid`
        (`/Game/UI/HUD/WBP_HUD.LadderInteractionLeave` (`self.As WBP HUD`))))))

(fn `UserConstructionScript`)